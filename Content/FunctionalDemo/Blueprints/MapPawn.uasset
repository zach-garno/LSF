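; MapPawn is a pawn for the functional demo that jumps between placed actors in its Levels array.
; It teleports to the first entry's location on BeginPlay.
; CycleForward and CycleBack inputs step the CurrentLevel index with wraparound and move the pawn to that actor's location.
; The backward move indexes with the decremented value rather than the wrapped CurrentLevel, so wrapping from the first entry uses an invalid index.
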(event EventBeginPlay
  (Transformation|SetActorLocation (Transformation|GetActorLocation (Utilities|Array|Get(acopy) (Variables|Default|GetLevels))) false false))

(event Collision|EventActorBeginOverlap
  (params (OtherActor :type Actor%20Object%20Reference)))

(event EventTick
  (params (DeltaSeconds :type Float%20%28single-precision%29)))

(event Input|ActionEvents|InputActionCycleForward
  (params (Key :type Key%20Structure))
  (bind _levels (Variables|Default|GetLevels))
  (:Pressed
    (bind _result (Math|Integer|IncrementInt (Variables|Default|GetCurrentLevel))
      (:%20%20
        (if (>= _result (Utilities|Array|Length _levels))
          (Variables|Default|SetCurrentLevel 0))
        (Transformation|SetActorLocation (Transformation|GetActorLocation (Utilities|Array|Get(acopy) _levels (Variables|Default|GetCurrentLevel))) false false)))))

(event Input|ActionEvents|InputActionCycleBack
  (params (Key :type Key%20Structure))
  (bind _levels (Variables|Default|GetLevels))
  (:Pressed
    (bind _result (Math|Integer|DecrementInt (Variables|Default|GetCurrentLevel))
      (:%20%20
        (if (> 0 _result)
          (Variables|Default|SetCurrentLevel (- (Utilities|Array|Length _levels) 1)))
        (Transformation|SetActorLocation (Transformation|GetActorLocation (Utilities|Array|Get(acopy) _levels _result)) false false)))))

(fn ConstructionScript)